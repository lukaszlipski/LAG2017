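; BP_Desk is a desk actor with a shelf that toggles open and closed.
; BeginPlay stores the starting relative locations of two static meshes.
; ToggleShelf checks and flips IsOpen, calling OpenShelfEvent or CloseShelfEvent.
; Opening plays Timeline_0 to slide both meshes along negative X from their stored positions, while closing calls Reverse on Timeline0.
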(event Custom|OpenShelfEvent
  (bind _newtrack_0 (Timeline|Timeline_0 Play)
    (:Update
      (Transformation|SetRelativeLocation (Variables|Default|GetStaticMesh1) (- (Variables|Default|Get1) (Math|Vector|MakeVector (* _newtrack_0 2e+01) 0.0 0.0)) false false)
      (Transformation|SetRelativeLocation (Variables|Default|GetStaticMesh2) (- (Variables|Default|Get2) (Math|Vector|MakeVector (* _newtrack_0 2e+01) 0.0 0.0)) false false))))

(event Custom|CloseShelfEvent
  (Utilities|String|Reverse (Variables|Default|GetTimeline_0)))

(event EventBeginPlay
  (Variables|Default|Set1 (Variables|/Script/Engine.SceneComponent|GetRelativeLocation (Variables|Default|GetStaticMesh1)))
  (Variables|Default|Set2 (Variables|/Script/Engine.SceneComponent|GetRelativeLocation (Variables|Default|GetStaticMesh2))))

(event Collision|EventActorBeginOverlap
  (params (OtherActor :type Actor%20Object%20Reference)))

(event EventTick
  (params (DeltaSeconds :type Float%20%28single-precision%29)))

(fn ConstructionScript)

(fn ToggleShelf
  (if (Variables|Default|GetIsOpen)
    (CallFunction|CloseShelfEvent)
    (Variables|Default|SetIsOpen false)
    (else
      (CallFunction|OpenShelfEvent)
      (Variables|Default|SetIsOpen true))))