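; BP_Paper is a noise distraction object that draws nearby AI to where it hits.
; Its first two hits spawn a puff effect, play an attenuated impact sound and call GoToPaper on BP_BasicAI actors found by a multi-sphere trace around the impact.
; A counter and the FirstHit flag silence later hits.
; A timeline started on BeginPlay acts as the lifetime, destroying the actor when it finishes.
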(event EventTick
  (params (DeltaSeconds :type Float%20%28single-precision%29)))

(event EventBeginPlay
  (Timeline|Timeline_0 Play
    (:Finished
      (Actor|DestroyActor))))

(event Collision|EventHit
  (params (MyComp :type Primitive%20Component%20Object%20Reference) (Other :type Actor%20Object%20Reference) (OtherComp :type Primitive%20Component%20Object%20Reference) (bSelfMoved :type Boolean) (HitLocation :type Vector) (HitNormal :type Vector) (NormalImpulse :type Vector) (Hit :type Hit%20Result%20Structure%20%28by%20ref%29))
  (if (Variables|Default|GetfirstHit)
    (bind _outhits (Collision|MultiSphereTraceByChannel HitLocation (+ HitLocation "0, 0,0.100000") (Variables|Default|Getradius) "TraceTypeQuery1" false 0 "None"))
    (Variables|Default|Setcounter (+ (Variables|Default|Getcounter) 1))
    (if (< (Variables|Default|Getcounter) 3)
      (Effects|SpawnEmitteratLocation "/Game/PUFF_Actor/PS_Puff.PS_Puff" (+ HitLocation (* HitNormal 5e+01)) "0, 0,0.000000")
      (Audio|PlaySoundatLocation "/Game/Sounds/PaperHit/a_Paper_Hit_01.a_Paper_Hit_01" HitLocation "0, 0, 0" 2.0 1.0 0.0 "/Game/Sounds/FootstepSoundAttenuation.FootstepSoundAttenuation")
      (for _array_element _outhits
        (bind _asbp_basic_ai (Utilities|Casting|CastToBP_BasicAI (.HitActor (Collision|BreakHitResult _array_element))))
        (Default|GotoPaper _asbp_basic_ai HitLocation))
      (else
        (Variables|Default|SetfirstHit false)))))

(fn ConstructionScript)