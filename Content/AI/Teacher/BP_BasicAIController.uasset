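; AI controller for the teacher NPC that catches the player, ending the game when it spots them in the open within range.
; PawnSensing sightings feed LookForPlayer, which line-traces on Visibility from player to AI and treats a BP_HideObject hit as hidden.
; Any other hit within LengthVisibility triggers GameOver, which stops movement and passes the controlled BP_BasicAI to the FirstPersonCharacter's own GameOver.
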(event OnSeePawn(PawnSensing)
  (params (Pawn :type Pawn%20Object%20Reference))
  (CallFunction|LookforPlayer Pawn))

(event EventTick
  (params (DeltaSeconds :type Float%20%28single-precision%29)))

(fn ConstructionScript)

(fn GameOver
  (AI|Navigation|StopMovement)
  (Development|PrintString "Game Over")
  (Default|GameOver (.AsFirst%20Person%20Character (Utilities|Casting|CastToFirstPersonCharacter (Game|Player|GetPlayerPawn 0))) (.AsBP%20Basic%20AI (Utilities|Casting|CastToBP_BasicAI (Pawn|GetControlledPawn)))))

(fn LookforPlayer
  (params (Object :type Object%20Object%20Reference))
  (bind _asfirst_person_character (Utilities|Casting|CastToFirstPersonCharacter Object))
  (LocalVariables|SetPlayer _asfirst_person_character)
  (bind (_outhit _returnvalue) (Collision|LineTraceByChannel (Transformation|GetActorLocation _asfirst_person_character) (Transformation|GetActorLocation (Pawn|GetControlledPawn)) "TraceTypeQuery1" false 0 "None"))
  (if _returnvalue
    ;[1 1 1] Is player behind object
    (Utilities|Casting|CastToBP_HideObject (.HitActor (Collision|BreakHitResult _outhit))
      (:then
        (Development|PrintString "UKRYTY" true true "(R=0.000000,G=0.660000,B=1.000000,A=1.000000)" 2.0))
      (:CastFailed
        (if (< (Math|Vector|VectorLength (- (Transformation|GetActorLocation (Pawn|GetControlledPawn)) (Transformation|GetActorLocation (LocalVariables|GetPlayer)))) (Variables|Default|GetLengthVisibility))
          ;[1 1 1] Player is visible for AI
          (CallFunction|GameOver))))))