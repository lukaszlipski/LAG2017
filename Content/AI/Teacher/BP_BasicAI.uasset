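; Teacher AI pawn, drawn as a billboard sprite, that walks to its current marker and can be diverted to a paper hit location.
; GoToPaper moves it near the hit, then it returns to the marker, pausing first on success.
; Tick turns the plane toward the player and picks a directional texture by comparing both facings, forcing Forward on game over.
; Tick also plays delayed footstep sounds while moving.
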(event Custom|GoToLocation
  (params (Hit%20 :type Vector))
  (bind _self self)
  (AI|AIMoveTo _self (.RandomLocation (AI|Navigation|GetRandomReachablePointinRadius Hit%20 0.0)) 0 2e+02 false
    (:OnSuccess
      (Utilities|FlowControl|Delay 2.0))
    (:OnFail
      _))
  (AI|Navigation|MovetoActor (AI|GetAIController _self) (Variables|Default|GetCurrentMarker) 3.0 true true))

(event EventBeginPlay
  (CallFunction|GotoMarker)
  (bind _returnvalue (Rendering|Material|CreateDynamicMaterialInstance (Variables|Default|GetPlane) 0 "/Game/AI/Teacher/M_Teacher_Inst.M_Teacher_Inst" :!class /Script/Engine.PrimitiveComponent))
  (Variables|Default|SetMaterialInstance _returnvalue))

(event EventTick
  (params (DeltaSeconds :type Float%20%28single-precision%29))
  (bind _returnvalue (Game|Player|GetPlayerPawn 0))
  (bind _returnvalue_2 (Game|Player|GetPlayerPawn 0))
  (bind _returnvalue_3 (Transformation|GetActorLocation))
  (bind _returnvalue_4 (Game|Player|GetPlayerPawn 0))
  (bind _materialinstance (Variables|Default|GetMaterialInstance))
  (bind _scene (Variables|Default|GetScene))
  (bind _materialinstance_2 (Variables|Default|GetMaterialInstance))
  (bind _materialinstance_3 (Variables|Default|GetMaterialInstance))
  (bind _materialinstance_4 (Variables|Default|GetMaterialInstance))
  (bind _materialinstance_5 (Variables|Default|GetMaterialInstance))
  (bind _returnvalue_5 (Math|Vector|GetForwardVector _scene))
  (bind _returnvalue_6 (Transformation|GetActorLocation _returnvalue))
  (bind _returnvalue_7 (Transformation|GetActorForwardVector _returnvalue_2))
  (bind _returnvalue_8 (Math|Vector|GetRightVector _scene))
  (bind _returnvalue_9 (Transformation|GetActorForwardVector _returnvalue_4))
  (bind _returnvalue_10 (Math|Vector|DotProduct _returnvalue_7 _returnvalue_5))
  (bind _returnvalue_11 (Math|Rotator|FindLookatRotation _returnvalue_3 _returnvalue_6))
  (bind _returnvalue_12 (Math|Vector|DotProduct _returnvalue_8 _returnvalue_9))
  (bind (_roll _pitch _yaw) (Math|Rotator|BreakRotator _returnvalue_11))
  (Utilities|FlowControl|Sequence
    (:then_0
      (Transformation|SetWorldRotation (Variables|Default|GetPlane) (Math|Rotator|CombineRotators (Math|Rotator|MakeRotator 9e+01 _pitch _yaw) "0,-90.000000, 0") false false)
      (bind _asfirst_person_character (Utilities|Casting|CastToFirstPersonCharacter _returnvalue_2)
        (:then
          (if (Variables|/Game/FirstPersonBP/Blueprints/FirstPersonCharacter.FirstPersonCharacter_C|GetbIsGameOver _asfirst_person_character)
            (Rendering|Material|SetTextureParameterValue _materialinstance_5 "TO" (Variables|Default|GetForward))
            (Rendering|Material|SetScalarParameterValue _materialinstance_5 "Poses" 2.0 :!class /Script/Engine.MaterialInstanceDynamic)
            (else
              (switch int (.IndexOfMinValue (Math|Float|MinOfFloatArray (Utilities|Array|MakeArray (Math|Float|Absolute(Float) (- _returnvalue_10 1.0)) (Math|Float|Absolute(Float) (- _returnvalue_10 -1.0)) (Math|Float|Absolute(Float) (- _returnvalue_12 1.0)) (Math|Float|Absolute(Float) (- _returnvalue_12 -1.0)))))
                (:0
                  (Rendering|Material|SetTextureParameterValue _materialinstance_2 "TO" (Variables|Default|GetBack))
                  (Rendering|Material|SetScalarParameterValue _materialinstance_2 "Poses" 2.0 :!class /Script/Engine.MaterialInstanceDynamic))
                (:1
                  (Rendering|Material|SetTextureParameterValue _materialinstance_3 "TO" (Variables|Default|GetForward))
                  (Rendering|Material|SetScalarParameterValue _materialinstance_3 "Poses" 2.0 :!class /Script/Engine.MaterialInstanceDynamic))
                (:2
                  (Rendering|Material|SetTextureParameterValue _materialinstance_4 "TO" (Variables|Default|GetLeft))
                  (Rendering|Material|SetScalarParameterValue _materialinstance_4 "Poses" 4.0 :!class /Script/Engine.MaterialInstanceDynamic))
                (:3
                  (Rendering|Material|SetTextureParameterValue _materialinstance "TO" (Variables|Default|GetRight))
                  (Rendering|Material|SetScalarParameterValue _materialinstance "Poses" 4.0 :!class /Script/Engine.MaterialInstanceDynamic))))))
        (:CastFailed
          (Development|PrintString "CANNOT CAST FirstPersonCharacter in BP_BasicAI::Tick" true true "(R=1.000000,G=0.000000,B=0.067137,A=1.000000)"))))
    (:then_1
      (if (> (Math|Vector|VectorLength (Transformation|GetVelocity)) 0.0)
        (Utilities|FlowControl|Delay 0.5)
        (if (> (Math|Vector|VectorLength (Transformation|GetVelocity)) 0.0)
          (Audio|PlaySoundatLocation "/Game/Sounds/Footstep/a_footstep_l_01_Cue.a_footstep_l_01_Cue" (Transformation|GetActorLocation) "0, 0, 0" 0.5 1.0 0.0 (Variables|Default|GetNewVar_0)))))))

(fn ConstructionScript)

(fn GotoMarker
  (AI|Navigation|MovetoActor (AI|GetAIController self) (Variables|Default|GetCurrentMarker) -1.0 true true))

(fn GotoPaper
  (params (Hit%20Location :type Vector))
  (CallFunction|GotoLocation Hit%20Location))