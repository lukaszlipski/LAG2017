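; BP_Widget is a 3D HUD widget actor whose Plane always turns to face the first-person player's camera.
; Each Tick, it takes the pitch and yaw of a look-at rotation from the actor to the camera and combines them with fixed offsets to orient the Plane.
; When any actor overlaps it, it destroys itself if the ShouldDisapear flag is set.
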(event EventBeginPlay)

(event Collision|EventActorBeginOverlap
  (params (OtherActor :type Actor%20Object%20Reference))
  (if (Variables|Default|GetbShouldDisapear)
    (Actor|DestroyActor)))

(event EventTick
  (params (DeltaSeconds :type Float%20%28single-precision%29))
  (bind _returnvalue (Game|Player|GetPlayerPawn 0))
  (bind _returnvalue_2 (Transformation|GetActorLocation))
  (bind _asfirst_person_character (Utilities|Casting|CastToFirstPersonCharacter _returnvalue))
  (bind _firstpersoncamera (Variables|/Game/FirstPersonBP/Blueprints/FirstPersonCharacter.FirstPersonCharacter_C|GetFirstPersonCamera _asfirst_person_character))
  (bind _returnvalue_3 (Transformation|GetWorldLocation _firstpersoncamera))
  (bind _returnvalue_4 (Math|Rotator|FindLookatRotation _returnvalue_2 _returnvalue_3))
  (bind (_roll _pitch _yaw) (Math|Rotator|BreakRotator _returnvalue_4))
  (Transformation|SetWorldRotation (Variables|Default|GetPlane) (Math|Rotator|CombineRotators (Math|Rotator|MakeRotator 9e+01 _pitch _yaw) "0,-90.000000, 0") false false))

(fn ConstructionScript)