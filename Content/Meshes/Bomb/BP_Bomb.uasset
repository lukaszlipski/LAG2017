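; Bomb actor with a hinged, toggleable door that leads into the player's bomb minigame.
; ToggleDoor flips IsOpen and calls OpenDoor or CloseDoor.
; OpenDoor plays a timeline that lerps StaticMesh1 from its BeginPlay rotation to EndRot, then calls OpenBombMiniGame on the FirstPersonCharacter when finished.
; CloseDoor calls Reverse on Timeline0, named differently from the Timeline_0 that drives opening.
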(event Custom|OpenDoor
  (bind _newtrack_0 (Timeline|Timeline_0 Play)
    (:Update
      (Transformation|SetRelativeRotation (Variables|Default|GetStaticMesh1) (Math|Rotator|Lerp(Rotator) (Variables|Default|GetStartRoot) (Variables|Default|GetEndRot) _newtrack_0) false false))
    (:Finished
      (Default|OpenBombMiniGame (.AsFirst%20Person%20Character (Utilities|Casting|CastToFirstPersonCharacter (Game|Player|GetPlayerPawn 0)))))))

(event Custom|CloseDoor
  (Utilities|String|Reverse (Variables|Default|GetTimeline_0)))

(event EventBeginPlay
  (Variables|Default|SetStartRoot (Variables|/Script/Engine.SceneComponent|GetRelativeRotation (Variables|Default|GetStaticMesh1))))

(event Collision|EventActorBeginOverlap
  (params (OtherActor :type Actor%20Object%20Reference)))

(event EventTick
  (params (DeltaSeconds :type Float%20%28single-precision%29)))

(fn ConstructionScript)

(fn ToggleDoor
  (if (Variables|Default|GetisOpen)
    (CallFunction|CloseDoor)
    (Variables|Default|SetisOpen false)
    (else
      (CallFunction|OpenDoor)
      (Variables|Default|SetisOpen true))))