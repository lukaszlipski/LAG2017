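; Door actor that swings its static mesh open and shut, with a locked state controlled by CanUOpenIt and NeedAKey.
; ToggleDoor alternates the open and close events, flips IsOpen and destroys the Widget actor if valid.
; A timeline drives the mesh's relative rotation and plays in reverse to close.
; The sound plays and IsOpen flips even when the lock check blocks opening.
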(event Custom|CloseDoorEvent
  (Audio|PlaySound2D "/Game/Sounds/Door/a_Door_Open_01.a_Door_Open_01")
  (Utilities|String|Reverse (Variables|Default|GetOpenDoorTimeline)))

(event Custom|OpenDoorEvent
  (Audio|PlaySound2D "/Game/Sounds/Door/a_Door_Open_01.a_Door_Open_01")
  (if (and (Variables|Default|GetCanUOpenIt) (not (Variables|Default|GetNeedAKey)))
    (bind _rotation (Timeline|OpenDoorTimeline Play)
      (:Update
        (Transformation|SetRelativeRotation (Variables|Default|GetStaticMesh) (Math|Rotator|CombineRotators (* (Math|Rotator|MakeRotator 0.0 9e+01 0.0) _rotation) "0, 0,90.000000") false false)))))

(event EventBeginPlay)

(event Collision|EventActorBeginOverlap
  (params (OtherActor :type Actor%20Object%20Reference)))

(event EventTick
  (params (DeltaSeconds :type Float%20%28single-precision%29)))

(fn ConstructionScript
  (|CallParentFunction))

(fn ToggleDoor
  (bind _widget (Variables|Default|GetWidget))
  (if (Variables|Default|GetIsOpen)
    (CallFunction|CloseDoorEvent)
    (Variables|Default|SetIsOpen false)
    (Utilities|IsValid _widget
      (:Is%20Valid
        (Actor|DestroyActor _widget)))
    (else
      (CallFunction|OpenDoorEvent)
      (Variables|Default|SetIsOpen true)
      (Utilities|IsValid _widget
        (:Is%20Valid
          (Actor|DestroyActor _widget))))))